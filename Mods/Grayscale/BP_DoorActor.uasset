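; BP_DoorActor is a usable door that swings open and closed when a player uses it.
; On BeginPlay it assigns the Door2 mesh to its static mesh component.
; Each use alternates through a FlipFlop between playing and reversing the DoorRotation timeline, whose track drives the mesh's relative yaw.
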(event `self.ReceiveBeginPlay`
  (`parent.ReceiveBeginPlay`)
  (`StaticMeshComponent.SetStaticMesh` (`self.StaticMesh`) "/Game/Mods/Grayscale/Models/BlackDoor/Door2.Door2"))

(event `self.ReceiveActorBeginOverlap`
  (params (OtherActor :type "Actor Object Reference"))
  (`parent.ReceiveActorBeginOverlap` OtherActor))

(event `self.OnActorUsed`
  (params (Character :type "Character Object Reference"))
  (`/Engine/EditorBlueprintResources/StandardMacros.FlipFlop`
    (:`A`
      (bind (_direction _doorrotationtrack) (`Timeline|DoorRotation` :!label _label)
        (:`Update`
          (`SceneComponent.K2_SetRelativeRotation` (`self.StaticMesh`) (`KismetMathLibrary.MakeRotator` 0.0 0.0 _doorrotationtrack) false false))))
    (:`B`
      (goto _label :!via `Reverse`))))

(fn `UserConstructionScript`
  (`parent.UserConstructionScript`))